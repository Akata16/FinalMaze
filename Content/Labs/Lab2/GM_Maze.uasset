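; GM_Maze is the maze lab's game mode, which sets up the on-screen HUD when play begins.
; BeginPlay creates the time and health bar widgets, stores a reference to each and adds both to the viewport.
; TimeUpdate returns the given timer value plus a fixed increment without storing it, and GetInteractState always returns false.
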(event EventBeginPlay
  (bind _returnvalue (UserInterface|CreateWidget "/Game/Labs/Lab3/W_Time.W_Time_C"))
  (Variables|Default|SetWidgetRef _returnvalue)
  (UserInterface|Viewport|AddtoViewport (Variables|Default|GetWidgetRef) 0)
  (bind _returnvalue_2 (UserInterface|CreateWidget "/Game/Labs/Lab3/W_HealthBar.W_HealthBar_C"))
  (bind _output_get (Variables|Default|SetHealthBarWidget _returnvalue_2))
  (UserInterface|Viewport|AddtoViewport _output_get 0))

(fn ConstructionScript)

(fn TimeUpdate
  (params (Timer :type Float%20%28double-precision%29))
  (return (+ Timer 15.0)))

(fn GetInteractState
  (return false))