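; BP_MazeCell is a configurable maze cell with optional walls, ceiling and a spike, axe or gas trap.
; The construction script scales the floor, adds meshes from grid size and wall height, sets the trap's child actor class and creates a downward spotlight.
; On BeginPlay, trapless cells roll to spawn a medkit, otherwise gold.
; A gate event registered with the player recolors the light to the player's color when IsInside is false.
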(event Custom|DP_Maze_Gate_Event
  (params (IsInside? :type Boolean))
  (bind _spotlight (Variables|Default|GetSpotLight))
  (if (not IsInside?)
    (Utilities|FlowControl|Delay 0.02)
    (Utilities|IsValid _spotlight
      (:Is%20Valid
        (Rendering|Components|Light|SetLightColor _spotlight (Variables|/Game/ThirdPerson/Blueprints/BP_ThirdPersonCharacter.BP_ThirdPersonCharacter_C|GetColor (Variables|Default|GetAs%20BP%20Third%20Person%20Character)) true)))))

(event EventBeginPlay
  (bind _scene (Variables|Default|GetScene))
  (bind _returnvalue (Transformation|GetWorldLocation _scene))
  (bind _asbp_third_person_character (Utilities|Casting|CastToBP_ThirdPersonCharacter (Game|GetPlayerCharacter 0)))
  (bind _output_get (Variables|Default|SetAs%20BP%20Third%20Person%20Character _asbp_third_person_character))
  (EventDispatchers|AssignDPMazeGate _output_get (delegate Custom|DP_Maze_Gate_Event))
  (if (not (Variables|Default|GetTrap))
    (if (>= (Math|Random|RandomIntegerinRange 0 10) 10)
      (Game|SpawnActorfromClass "/Game/Labs/Lab3/BP_Medkit.BP_Medkit_C" (Math|Transform|MakeTransform _returnvalue "0, 0, 0" "1.000000,1.000000,1.000000") "Undefined" "MultiplyWithRoot" 0 0)
      (elif (>= (Math|Random|RandomIntegerinRange 0 10) 10)
        (Game|SpawnActorfromClass "/Game/Labs/Lab2/BP_Gold.BP_Gold_C" (Math|Transform|MakeTransform _returnvalue "0, 0, 0" "1.000000,1.000000,1.000000") "Undefined" "MultiplyWithRoot" 0 0)))))

(event Collision|EventActorBeginOverlap
  (params (OtherActor :type Actor%20Object%20Reference)))

(event EventTick
  (params (DeltaSeconds :type Float%20%28single-precision%29)))

(fn ConstructionScript
  (bind _gridsize (Variables|Default|GetGridSize))
  (bind _wallheight (Variables|Default|GetWallHeight))
  (bind _childactor (Variables|Default|GetChildActor))
  (bind _returnvalue (* _wallheight 0.5))
  (LocalVariables|SetWallLength _gridsize)
  (LocalVariables|SetWallThickness (* _gridsize 0.1))
  (Transformation|SetRelativeScale3D (Variables|Default|GetFloor) (Utilities|CubeDimension (Math|Vector|MakeVector (LocalVariables|GetWallLength) (LocalVariables|GetWallLength) (LocalVariables|GetWallThickness))))
  (if (Variables|Walls|GetWestWall)
    (AddComponent|AddStaticMeshComponent false (Math|Transform|MakeTransform "0, 0, 0" "0, 0, 0" (Utilities|CubeDimension (Math|Vector|MakeVector (LocalVariables|GetWallLength) (LocalVariables|GetWallThickness) (Variables|Default|GetWallHeight))))))
  (if (Variables|Walls|GetSouthWall)
    (AddComponent|AddStaticMeshComponent false (Math|Transform|MakeTransform "0, 0, 0" "0, 0, 0" (Utilities|CubeDimension (Math|Vector|MakeVector (LocalVariables|GetWallThickness) (LocalVariables|GetWallLength) (Variables|Default|GetWallHeight))))))
  (if (Variables|Walls|GetEastWall)
    (AddComponent|AddStaticMeshComponent false (Math|Transform|MakeTransform (Math|Vector|MakeVector 0.0 (- (LocalVariables|GetWallLength) (LocalVariables|GetWallThickness)) 0.0) "0, 0, 0" (Utilities|CubeDimension (Math|Vector|MakeVector (LocalVariables|GetWallLength) (LocalVariables|GetWallThickness) (Variables|Default|GetWallHeight))))))
  (if (Variables|Walls|GetNorthWall)
    (AddComponent|AddStaticMeshComponent false (Math|Transform|MakeTransform (Math|Vector|MakeVector (- (LocalVariables|GetWallLength) (LocalVariables|GetWallThickness)) 0.0 0.0) "0, 0, 0" (Utilities|CubeDimension (Math|Vector|MakeVector (LocalVariables|GetWallThickness) (LocalVariables|GetWallLength) (Variables|Default|GetWallHeight))))))
  (if (Variables|Walls|GetCeiling)
    (AddComponent|AddStaticMeshComponent false (Math|Transform|MakeTransform (Math|Vector|MakeVector 0.0 0.0 (Variables|Default|GetWallHeight)) "0, 0, 0" (Utilities|CubeDimension (Math|Vector|MakeVector (LocalVariables|GetWallLength) (Variables|Default|GetWallHeight) (LocalVariables|GetWallThickness))))))
  (switch Utilities|FlowControl|Switch|SwitchonEnum_TrapType (Variables|Default|GetTrapType)
    (:NewEnumerator0
      (Variables|Default|SetTrap false))
    (:NewEnumerator1
      (Variables|Default|SetTrap true)
      (ChildActorComponent|SetChildActorClass (Variables|Default|GetChildActor) "/Game/Labs/Lab3/BP_SpikeTrap.BP_SpikeTrap_C")
      (if (> (Variables|Default|GetLightIntensity) 0.0) :!label _label
        _
        (else
          _)))
    (:NewEnumerator2
      (Variables|Default|SetTrap true)
      (ChildActorComponent|SetChildActorClass _childactor "/Game/Labs/Lab3/BP_AxeTrap.BP_AxeTrap_C")
      (Transformation|SetWorldRotation _childactor (Variables|Default|GetTrapRotation) false false)
      (goto _label))
    (:NewEnumerator3
      (Variables|Default|SetTrap true)
      (ChildActorComponent|SetChildActorClass (Variables|Default|GetChildActor) "/Game/Labs/Lab3/BP_GasTrap.BP_GasTrap_C")
      (goto _label)))
  (bind _returnvalue_2 (AddComponent|AddSpotLightComponent false (Math|Transform|MakeTransform (Math|Vector|MakeVector _returnvalue _returnvalue (Variables|Default|GetWallHeight)) "-90.000000,0.000000,0.000000" "1.000000,1.000000,1.000000")))
  (bind _output_get (Variables|Default|SetSpotLight _returnvalue_2))
  (Rendering|Components|Light|SetIntensity _output_get (Variables|Default|GetLightIntensity))
  (Rendering|Components|Light|SetLightColor _output_get (Variables|Default|GetNew%20Light%20Color) true))